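; WaveHUDB is the HUD Blueprint for the wave mission, showing how many enemies remain.
; On each DrawHUD it casts the game state to WaveGameStateB and draws text with NumberToWin minus NumberDestroyed.
; It draws directly on the HUD canvas rather than through widgets, and nothing draws if the cast fails.
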(event `self.ReceiveBeginPlay`)

(event `self.ReceiveActorBeginOverlap`
  (params (OtherActor :type "Actor Object Reference")))

(event `self.ReceiveTick`
  (params (DeltaSeconds :type "Float (single-precision)")))

(event `self.ReceiveDrawHUD`
  (params (SizeX :type Integer) (SizeY :type Integer))
  (`parent.ReceiveDrawHUD` 0 0)
  (bind _aswave_game_state_b (cast `/Game/Blueprints/WaveMission/WaveGameStateB` (`GameplayStatics.GetGameState`)))
  (`self.DrawText` (`KismetStringLibrary.Concat_StrStr` "Enemies Remaining: " (`KismetStringLibrary.Conv_IntToString` (- (`/Game/Blueprints/WaveMission/WaveGameStateB.NumberToWin` _aswave_game_state_b) (`/Game/Blueprints/WaveMission/WaveGameStateB.NumberDestroyed` _aswave_game_state_b)))) (struct :`A` 1) 0.0 0.0 "/Game/Fonts/Data.Data" 2.0))

(fn `UserConstructionScript`
  (`parent.UserConstructionScript`))