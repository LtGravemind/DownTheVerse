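; Wave mission drone fighter variant that registers as a target and counts toward the win condition when destroyed.
; On BeginPlay it adds itself to the TargetList on CombatGameState.
; On Destroyed it casts the game state to WaveGameStateB, removes itself from that TargetList and decrements NumberToWin.
; Construction only calls the parent script, and overlap and Tick events are disabled.
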(event `self.ReceiveBeginPlay`
  (bind _ascombat_game_state (cast `CombatGameState` (`GameplayStatics.GetGameState`)))
  (`KismetArrayLibrary.Array_Add` (`CombatGameState.TargetList` _ascombat_game_state) self))

(event `self.ReceiveActorBeginOverlap`
  (params (OtherActor :type "Actor Object Reference")))

(event `self.ReceiveTick`
  (params (DeltaSeconds :type "Float (single-precision)")))

(event `self.ReceiveDestroyed`
  (bind _aswave_game_state_b (cast `/Game/Blueprints/WaveMission/WaveGameStateB` (`GameplayStatics.GetGameState`)))
  (`KismetArrayLibrary.Array_RemoveItem` (`CombatGameState.TargetList` _aswave_game_state_b) self)
  (bind _aswave_game_state_b_2 (cast `/Game/Blueprints/WaveMission/WaveGameStateB` (`GameplayStatics.GetGameState`)))
  (set `/Game/Blueprints/WaveMission/WaveGameStateB.NumberToWin` (- (`/Game/Blueprints/WaveMission/WaveGameStateB.NumberToWin` _aswave_game_state_b_2) 1) _aswave_game_state_b_2))

(fn `UserConstructionScript`
  (`parent.UserConstructionScript`))