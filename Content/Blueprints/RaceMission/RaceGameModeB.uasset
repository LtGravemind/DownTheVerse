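; Game mode Blueprint for the race mission that lets the player quit to the level selection screen.
; On BeginPlay it runs the parent logic and enables input from the first player controller so it can receive key presses directly.
; Pressing Escape casts the active game mode to FighterGameModeB, removes its HUD widget and opens the LevelSelection level.
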(event `self.ReceiveBeginPlay`
  (`parent.ReceiveBeginPlay`)
  (`self.EnableInput` (`GameplayStatics.GetPlayerController` 0)))

(event `Key|Escape`
  (:`Pressed`
    (bind _asfighter_game_mode_b (cast `/Game/Blueprints/FighterMode/FighterGameModeB` (`GameplayStatics.GetGameMode`)))
    (`Widget.RemoveFromParent` (`/Game/Blueprints/FighterMode/FighterGameModeB.GameWidgetHUD` _asfighter_game_mode_b))
    (`GameplayStatics.OpenLevel` "LevelSelection")))

(fn `UserConstructionScript`
  (`parent.UserConstructionScript`))