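; Game state for the wave-based combat training mission, which spawns drones at a quickening pace and ends the mission on victory.
; Tick triggers every spawner in SpawnerList once the delay elapses, shortening it per spawner toward a minimum, until NumberSpawned reaches NumberToWin.
; When NumberDestroyed reaches that target, it records CombatTraining completion and experience in the game instance, removes the HUD and opens LevelSelection.
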(event `self.ReceiveBeginPlay`
  (set `self.Time` (`KismetSystemLibrary.GetGameTimeInSeconds`)))

(event `self.ReceiveTick`
  (params (DeltaSeconds :type "Float (single-precision)"))
  (bind _numbertowin (`self.NumberToWin`))
  (bind _returnvalue (- (`self.Delay`) (`self.DecrementDelayBy`)))
  (if (and (> (- (`KismetSystemLibrary.GetGameTimeInSeconds`) (`self.Delay`)) (`self.Time`)) (not (>= (`self.NumberSpawned`) _numbertowin)))
    (for _array_element (`self.SpawnerList`)
      (`/Game/Blueprints/WaveMission/WaveSpawnerB.SpawnDrone` _array_element)
      (if (not (< _returnvalue (`self.MinimumDelay`)))
        (set `self.Delay` _returnvalue))
      (set `self.Time` (`KismetSystemLibrary.GetGameTimeInSeconds`))
      (`KismetSystemLibrary.PrintString` "Enemy spawned." true true (struct :`R` 1.0 :`B` 0.054663 :`A` 1.0)))
    (elif (>= (`self.NumberDestroyed`) _numbertowin)
      (bind _asdown_the_verse_game_instance_b (cast `/Game/Blueprints/DownTheVerseGameInstanceB` (`GameplayStatics.GetGameInstance`)))
      (`KismetArrayLibrary.Array_Add` (`/Game/Blueprints/DownTheVerseGameInstanceB.CompletedLevels` _asdown_the_verse_game_instance_b) "CombatTraining")
      (bind _asdown_the_verse_game_instance_b_2 (cast `/Game/Blueprints/DownTheVerseGameInstanceB` (`GameplayStatics.GetGameInstance`)))
      (`/Game/Blueprints/DownTheVerseGameInstanceB.AddExperience` _asdown_the_verse_game_instance_b_2 100)
      (bind _asfighter_game_mode_b (cast `/Game/Blueprints/FighterMode/FighterGameModeB` (`GameplayStatics.GetGameMode`)))
      (`Widget.RemoveFromParent` (`/Game/Blueprints/FighterMode/FighterGameModeB.GameWidgetHUD` _asfighter_game_mode_b))
      (`GameplayStatics.OpenLevel` "LevelSelection"))))

(fn `UserConstructionScript`)