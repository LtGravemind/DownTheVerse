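; RaceHUDB is the HUD for a race mission, showing goals remaining, time remaining and a marker on the active goal.
; Each DrawHUD reads the counters from RaceGameStateB and draws them as text, with time formatted as a timespan.
; It projects the active goal's world location to screen space and draws a centered orange reticle, only when the goal is valid and in front of the camera.
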(event `self.ReceiveDrawHUD`
  (params (SizeX :type Integer) (SizeY :type Integer))
  (`parent.ReceiveDrawHUD` 0 0)
  (bind _asrace_game_state_b (cast `/Game/Blueprints/RaceMission/RaceGameStateB` (`GameplayStatics.GetGameState`)))
  (`self.DrawText` (`KismetStringLibrary.Concat_StrStr` "Goals Remaining: " (`KismetStringLibrary.Conv_IntToString` (`/Game/Blueprints/RaceMission/RaceGameStateB.GoalsRemaining` _asrace_game_state_b))) (struct :`A` 1) 0.0 0.0 "/Game/Fonts/Data.Data" 2.0)
  (`self.DrawText` (`KismetStringLibrary.Concat_StrStr` "Time Remaining: " (`KismetTextLibrary.Conv_TextToString` (`KismetTextLibrary.AsTimespan_Timespan` (`KismetMathLibrary.FromSeconds` (`/Game/Blueprints/RaceMission/RaceGameStateB.TimeRemaining` _asrace_game_state_b))))) (struct :`A` 1) 50.0 50.0 "/Game/Fonts/Data.Data" 2.0)
  (bind _activegoal (`/Game/Blueprints/RaceMission/RaceGameStateB.ActiveGoal` _asrace_game_state_b))
  (if (`KismetSystemLibrary.IsValid` _activegoal)
    (if (> (.z (`self.Project` (`self.K2_GetActorLocation` _activegoal))) 0.0)
      (`self.DrawTexture` "/Game/Materials/reticle.reticle" (- (.x (`self.Project` (`self.K2_GetActorLocation` _activegoal))) 25.0) (- (.y (`self.Project` (`self.K2_GetActorLocation` _activegoal))) 25.0) 50.0 50.0 0.0 0.0 1.0 1.0 (struct :`R` 1.0 :`G` 0.527411 :`A` 1.0)))))

(fn `UserConstructionScript`
  (`parent.UserConstructionScript`))