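; RaceGoalB is a numbered race goal actor for the race mission that must be the active goal to be cleared.
; On BeginPlay it inserts itself into RaceGameStateB's GoalList in GoalNumber order and increments GoalsRemaining.
; On any actor overlap while it is the game state's ActiveGoal, it decrements GoalsRemaining, removes itself from the list and destroys itself.
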(event `self.ReceiveBeginPlay`
  (bind _asrace_game_state_b (cast `/Game/Blueprints/RaceMission/RaceGameStateB` (`GameplayStatics.GetGameState`)))
  (bind _goallist (`/Game/Blueprints/RaceMission/RaceGameStateB.GoalList` _asrace_game_state_b))
  (for _index (range (`KismetArrayLibrary.Array_Length` _goallist))
    (if (<= (`self.GoalNumber`) (`/Game/Blueprints/RaceMission/RaceGoalB.GoalNumber` (`KismetArrayLibrary.Array_Get` _goallist _index)))
      (`KismetArrayLibrary.Array_Insert` _goallist self _index)
      (break)))
  (set `/Game/Blueprints/RaceMission/RaceGameStateB.GoalsRemaining` (+ 1 (`/Game/Blueprints/RaceMission/RaceGameStateB.GoalsRemaining` _asrace_game_state_b)) _asrace_game_state_b)
  (if (or (== (`KismetArrayLibrary.Array_Length` _goallist) 0) (not (`KismetArrayLibrary.Array_Contains` _goallist self)))
    (`KismetArrayLibrary.Array_Add` _goallist self)))

(event `self.ReceiveActorBeginOverlap`
  (params (OtherActor :type "Actor Object Reference"))
  (bind _asrace_game_state_b (cast `/Game/Blueprints/RaceMission/RaceGameStateB` (`GameplayStatics.GetGameState`)))
  (if (== (`/Game/Blueprints/RaceMission/RaceGameStateB.ActiveGoal` _asrace_game_state_b) self)
    (set `/Game/Blueprints/RaceMission/RaceGameStateB.GoalsRemaining` (- (`/Game/Blueprints/RaceMission/RaceGameStateB.GoalsRemaining` _asrace_game_state_b) 1) _asrace_game_state_b)
    (`KismetArrayLibrary.Array_RemoveItem` (`/Game/Blueprints/RaceMission/RaceGameStateB.GoalList` _asrace_game_state_b) self)
    (`self.K2_DestroyActor`)))

(fn `UserConstructionScript`)