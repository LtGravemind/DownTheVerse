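; Pawn for the level selection screen that the player moves across the map to pick and load a level.
; WASD or left stick set direction flags, and Tick applies a fixed per-frame world offset without sweep or delta-time scaling.
; Overlapping a LevelNodeB stores its display name, plus its level name if unlocked; leaving resets both.
; Left click or gamepad bottom face button removes the game mode's selection widget and opens the stored level.
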(event `Key|Gamepad_LeftStick_Up`
  (:`Pressed`
    (`self.Forward` true :!label _label))
  (:`Released`
    (`self.Forward` false :!label _label_2)))

(event `Key|W`
  (:`Pressed`
    (goto _label))
  (:`Released`
    (goto _label_2)))

(event `Key|Gamepad_LeftStick_Down`
  (:`Pressed`
    (`self.Back` true :!label _label_3))
  (:`Released`
    (`self.Back` false :!label _label_4)))

(event `Key|S`
  (:`Pressed`
    (goto _label_3))
  (:`Released`
    (goto _label_4)))

(event `self.ReceiveTick`
  (params (DeltaSeconds :type "Float (single-precision)"))
  (if (`self.IsWPressed`)
    (`self.K2_AddActorWorldOffset` (10.0 0.0 0.0)))
  (if (`self.IsAPressed`)
    (`self.K2_AddActorWorldOffset` (0.0 -10.0 0.0)))
  (if (`self.IsSPressed`)
    (`self.K2_AddActorWorldOffset` (-10.0 0.0 0.0)))
  (if (`self.IsDPressed`)
    (`self.K2_AddActorWorldOffset` (0.0 10.0 0.0))))

(event `Key|Gamepad_LeftStick_Left`
  (:`Pressed`
    (`self.Left` true :!label _label_5))
  (:`Released`
    (`self.Left` false :!label _label_6)))

(event `Key|A`
  (:`Pressed`
    (goto _label_5))
  (:`Released`
    (goto _label_6)))

(event `Key|D`
  (:`Pressed`
    (`self.Right` true :!label _label_7))
  (:`Released`
    (`self.Right` false :!label _label_8)))

(event `Key|Gamepad_LeftStick_Right`
  (:`Pressed`
    (goto _label_7))
  (:`Released`
    (goto _label_8)))

(event `Key|Gamepad_FaceButton_Bottom`
  (bind _levelselected (`self.LevelSelected`))
  (:`Pressed`
    (if (not (== "None" _levelselected)) :!label _label_9
      (bind _aslevel_selection_game_mode_b (cast `/Game/Blueprints/LevelSelection/LevelSelectionGameModeB` (`GameplayStatics.GetGameMode`)))
      (`Widget.RemoveFromParent` (`/Game/Blueprints/LevelSelection/LevelSelectionGameModeB.Level Select Widget` _aslevel_selection_game_mode_b))
      (`GameplayStatics.OpenLevel` _levelselected))))

(event `Key|LeftMouseButton`
  (:`Pressed`
    (goto _label_9)))

(event `self.ReceiveActorBeginOverlap`
  (params (OtherActor :type "Actor Object Reference"))
  (bind _aslevel_node_b (cast `/Game/Blueprints/LevelSelection/LevelNodeB` OtherActor))
  (if (`/Game/Blueprints/LevelSelection/LevelNodeB.IsUnlocked` _aslevel_node_b)
    (set `self.LevelSelected` (`/Game/Blueprints/LevelSelection/LevelNodeB.LevelName` _aslevel_node_b)))
  (set `self.LevelDisplayName` (`/Game/Blueprints/LevelSelection/LevelNodeB.DisplayName` _aslevel_node_b)))

(event `self.ReceiveActorEndOverlap`
  (params (OtherActor :type "Actor Object Reference"))
  (set `self.LevelSelected` "None")
  (set `self.LevelDisplayName` "None"))

(fn `Back`
  (params (IsPressed :type Boolean))
  (set `self.IsSPressed` IsPressed))

(fn `Forward`
  (params (IsPressed :type Boolean))
  (set `self.IsWPressed` IsPressed))

(fn `Left`
  (params (IsPressed :type Boolean))
  (set `self.IsAPressed` IsPressed))

(fn `Right`
  (params (IsPressed :type Boolean))
  (set `self.IsDPressed` IsPressed))

(fn `UserConstructionScript`)