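; MissileLauncherComponentB is a Fighter Mode component that launches guided missiles at the player's current target.
; FireMissile spawns a Missile at the component's world location and rotation, then sets its speed and a fixed lifespan.
; It reads CurrentTarget from the first player's CombatHUD and passes it to the missile; if the HUD cast fails, the missile still flies, with no target assigned.
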(event `self.ReceiveTick`
  (params (DeltaSeconds :type "Float (single-precision)")))

(event `self.ReceiveInitializeComponent`)

(fn `FireMissile`
  (bind _returnvalue (`|SpawnActorFromClass` "/Script/DownTheVerse.Missile" (`KismetMathLibrary.MakeTransform` (`self.K2_GetComponentLocation`) (`self.K2_GetComponentRotation`))))
  (`Missile.SetCurrentSpeed` _returnvalue (`self.Speed`))
  (`Actor.SetLifeSpan` _returnvalue 10.0)
  (bind _ascombat_hud (cast `CombatHUD` (`PlayerController.GetHUD` (`GameplayStatics.GetPlayerController` 0))))
  (`Missile.SetCurrentTarget` _returnvalue (`CombatHUD.CurrentTarget` _ascombat_hud)))