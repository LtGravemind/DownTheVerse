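; Laser weapon component for Fighter Mode that fires an instant hitscan shot, damaging the first object hit.
; FireLaser runs an object-type line trace from the owner's location along its forward vector, ignoring the owner, then applies damage on a hit.
; The visible beam is a short-lived debug line from the component's location, ending at the impact point or, on a miss, at range along the component's own forward vector.
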(event EventTick
  (params (DeltaSeconds :type Float%20%28single-precision%29)))

(event EventInitializeComponent)

(fn FireLaser
  (bind _returnvalue (Components|GetOwner))
  (bind _returnvalue_2 (Transformation|GetWorldLocation))
  (bind _lasercolor (Variables|Default|GetLaserColor))
  (bind _range (Variables|Default|GetRange))
  (bind _returnvalue_3 (Transformation|GetActorLocation _returnvalue))
  (bind (_outhit _returnvalue_4) (Collision|LineTraceForObjects _returnvalue_3 (+ _returnvalue_3 (* (Math|Vector|GetForwardVector (Transformation|GetActorRotation _returnvalue)) _range)) (LocalVariables|GetHitTypes) false (Utilities|Array|MakeArray (Components|GetOwner) 0) "None"))
  (if _returnvalue_4
    (Rendering|Debug|DrawDebugLine _returnvalue_2 (.ImpactPoint (Collision|BreakHitResult _outhit)) _lasercolor 0.25 3.5)
    (Game|Damage|ApplyDamage (.HitActor (Collision|BreakHitResult _outhit)) (Variables|Default|GetDamage) 0 0)
    (else
      (Rendering|Debug|DrawDebugLine _returnvalue_2 (+ _returnvalue_2 (* (Math|Vector|GetForwardVector (Transformation|GetWorldRotation)) _range)) _lasercolor 0.25 3.5))))