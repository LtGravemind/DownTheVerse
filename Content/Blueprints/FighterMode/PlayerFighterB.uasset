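; Player-controlled fighter for Fighter Mode that fires lasers and missiles with sound effects.
; On BeginPlay it copies max health, max speed and acceleration from DownTheVerseGameInstanceB and starts audio, which replays whenever it finishes.
; Left mouse or right trigger calls FireLaser twice, while right mouse or left trigger calls FireMissile.
; A second right-trigger binding plays the laser sound again.
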(event `self.ReceiveBeginPlay`
  (`AudioComponent.Play` 0.0)
  (bind _asdown_the_verse_game_instance_b (cast `/Game/Blueprints/DownTheVerseGameInstanceB` (`GameplayStatics.GetGameInstance`)))
  (set `self.MaxHealth` (`/Game/Blueprints/DownTheVerseGameInstanceB.PlayerMaxHealth` _asdown_the_verse_game_instance_b))
  (set `self.MaxSpeed` (`/Game/Blueprints/DownTheVerseGameInstanceB.PlayerMaxSpeed` _asdown_the_verse_game_instance_b))
  (set `self.Acceleration` (`/Game/Blueprints/DownTheVerseGameInstanceB.PlayerAcceleration` _asdown_the_verse_game_instance_b)))

(event `Key|Gamepad_RightTrigger`
  (:`Pressed`
    (`GameplayStatics.PlaySoundAtLocation` "/Game/Sounds/laser.laser" (`self.K2_GetActorLocation`))))

(event `self.Audio.OnAudioFinished`
  (`AudioComponent.Play` 0.0))

(event `Key|LeftMouseButton`
  (:`Pressed`
    (`/Game/Blueprints/FighterMode/LaserComponentB.FireLaser`)
    (`/Game/Blueprints/FighterMode/LaserComponentB.FireLaser`)
    (`GameplayStatics.PlaySoundAtLocation` "/Game/Sounds/laser.laser" (`self.K2_GetActorLocation`))))

(event `Key|RightMouseButton`
  (:`Pressed`
    (`/Game/Blueprints/FighterMode/MissileLauncherComponentB.FireMissile`)
    (`GameplayStatics.PlaySoundAtLocation` "/Game/Sounds/missile.missile" (`self.K2_GetActorLocation`))))

(event `Key|Gamepad_RightTrigger`
  (:`Pressed`
    (`/Game/Blueprints/FighterMode/LaserComponentB.FireLaser`)
    (`/Game/Blueprints/FighterMode/LaserComponentB.FireLaser`)
    (`GameplayStatics.PlaySoundAtLocation` "/Game/Sounds/laser.laser" (`self.K2_GetActorLocation`))))

(event `Key|Gamepad_LeftTrigger`
  (:`Pressed`
    (`/Game/Blueprints/FighterMode/MissileLauncherComponentB.FireMissile`)
    (`GameplayStatics.PlaySoundAtLocation` "/Game/Sounds/missile.missile" (`self.K2_GetActorLocation`))))

(fn `UserConstructionScript`)