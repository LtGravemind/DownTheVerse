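; Game instance for DownTheVerse that tracks the player's current XP and level.
; AddExperience adds to CurrentXP, then walks every row of the XPTable data table and compares the total with each RequiredXP.
; Row names double as level numbers, so CurrentLevel becomes the last qualifying row's name converted to an integer, which relies on ascending row order.
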(fn `AddExperience`
  (params (Experience :type Integer))
  (set `self.CurrentXP` (+ Experience (`self.CurrentXP`)))
  (bind _outrownames (`DataTableFunctionLibrary.GetDataTableRowNames` "/Game/Data/XPTable.XPTable"))
  (for _array_element _outrownames
    (bind _returnvalue (`|GetDataTableRow` "/Game/Data/XPTable.XPTable" _array_element)
      (:`then`
        (if (>= (`self.CurrentXP`) (`.RequiredXP` (break `XPTable` _returnvalue)))
          (set `self.CurrentLevel` (`KismetStringLibrary.Conv_StringToInt` (`KismetStringLibrary.Conv_NameToString` _array_element))))))))