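; Game state for the race mission that runs a countdown and decides when the race is won or lost.
; Each tick it lowers the remaining time and, when the active goal is invalid, takes the first entry in the goal list.
; No valid goal with time left records RaceTraining as completed on the game instance and awards experience.
; Both success and timeout remove the HUD and open the level selection map.
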(event `self.ReceiveTick`
  (params (DeltaSeconds :type "Float (single-precision)"))
  (bind _timeremaining (`self.TimeRemaining`))
  (bind _returnvalue (> (`self.TimeRemaining`) 0.0))
  (if (>= _timeremaining 0.0)
    (set `self.TimeRemaining` (- _timeremaining DeltaSeconds))
    (if (not (`KismetSystemLibrary.IsValid` (`self.ActiveGoal`)))
      (bind _output_get (set `self.ActiveGoal` (`KismetArrayLibrary.Array_Get` (`self.GoalList`)))))
    (if (and (not (`KismetSystemLibrary.IsValid` _output_get)) _returnvalue)
      (bind _asdown_the_verse_game_instance_b (cast `/Game/Blueprints/DownTheVerseGameInstanceB` (`GameplayStatics.GetGameInstance`)))
      (`KismetArrayLibrary.Array_Add` (`/Game/Blueprints/DownTheVerseGameInstanceB.CompletedLevels` _asdown_the_verse_game_instance_b) "RaceTraining")
      (bind _asdown_the_verse_game_instance_b_2 (cast `/Game/Blueprints/DownTheVerseGameInstanceB` (`GameplayStatics.GetGameInstance`)))
      (`/Game/Blueprints/DownTheVerseGameInstanceB.AddExperience` _asdown_the_verse_game_instance_b_2 500)
      (bind _asfighter_game_mode_b (cast `/Game/Blueprints/FighterMode/FighterGameModeB` (`GameplayStatics.GetGameMode`) :!label _label))
      (`Widget.RemoveFromParent` (`/Game/Blueprints/FighterMode/FighterGameModeB.GameWidgetHUD` _asfighter_game_mode_b))
      (`GameplayStatics.OpenLevel` "LevelSelection")
      (elif (not _returnvalue)
        (goto _label)))))

(fn `UserConstructionScript`)