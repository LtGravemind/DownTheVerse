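; Behemoth is a boss fight actor that slowly rotates to face the player every tick while its guns remain.
; GunsLeft starts as the count of child components; this graph never decrements it.
; When it reaches zero with a valid player, the boss destroys itself, awards experience through the game instance, removes the HUD, records BossTraining as completed and opens the LevelSelection level.
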(event `self.ReceiveBeginPlay`
  (set `self.GunsLeft` (`SceneComponent.GetNumChildrenComponents`)))

(event `self.ReceiveTick`
  (params (DeltaSeconds :type "Float (single-precision)"))
  (bind _returnvalue (`GameplayStatics.GetPlayerPawn` 0))
  (if (`KismetSystemLibrary.IsValid` _returnvalue)
    (if (== (`self.GunsLeft`) 0)
      (`self.K2_DestroyActor`)
      (bind _asdown_the_verse_game_instance_b (cast `/Game/Blueprints/DownTheVerseGameInstanceB` (`GameplayStatics.GetGameInstance`)))
      (`/Game/Blueprints/DownTheVerseGameInstanceB.AddExperience` _asdown_the_verse_game_instance_b 1000)
      (bind _asfighter_game_mode_b (cast `/Game/Blueprints/FighterMode/FighterGameModeB` (`GameplayStatics.GetGameMode`)))
      (`Widget.RemoveFromParent` (`/Game/Blueprints/FighterMode/FighterGameModeB.GameWidgetHUD` _asfighter_game_mode_b))
      (bind _asdown_the_verse_game_instance_b_2 (cast `/Game/Blueprints/DownTheVerseGameInstanceB` (`GameplayStatics.GetGameInstance`)))
      (`KismetArrayLibrary.Array_Add` (`/Game/Blueprints/DownTheVerseGameInstanceB.CompletedLevels` _asdown_the_verse_game_instance_b_2) "BossTraining")
      (`GameplayStatics.OpenLevel` "LevelSelection")
      (else
        (`self.SetActorRotation` (`KismetMathLibrary.RInterpTo_Constant` (`self.K2_GetActorRotation`) (`KismetMathLibrary.FindLookAtRotation` (`self.K2_GetActorLocation`) (`self.K2_GetActorLocation` _returnvalue)) DeltaSeconds 10.0))))))

(fn `UserConstructionScript`)