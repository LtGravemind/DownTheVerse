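; Destructible gun battery for the Behemoth boss fight that tracks and damages the player.
; Each tick it turns toward player pawn 0 at a constant rate and line-traces forward against WorldDynamic objects, ignoring its attach parent's owner.
; Hits take damage every frame, and the trace is debug-drawn.
; When its health runs out, it decrements GunsLeft on the parent Behemoth and destroys itself.
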(event `self.ReceiveTick`
  (params (DeltaSeconds :type "Float (single-precision)"))
  (bind _returnvalue (`GameplayStatics.GetPlayerPawn` 0))
  (bind _returnvalue_2 (`self.K2_GetActorLocation`))
  (if (`KismetSystemLibrary.IsValid` _returnvalue)
    (`self.SetActorRotation` (`KismetMathLibrary.RInterpTo_Constant` (`self.K2_GetActorRotation`) (`KismetMathLibrary.FindLookAtRotation` (`self.K2_GetActorLocation`) (`self.K2_GetActorLocation` _returnvalue)) DeltaSeconds 50.0))
    (bind (_outhit _returnvalue_3) (`KismetSystemLibrary.LineTraceSingleForObjects` _returnvalue_2 (+ (* (`KismetMathLibrary.GetForwardVector` (`self.K2_GetActorRotation`)) 5000.0) _returnvalue_2) (`|MakeArray` "ObjectTypeQuery2" :!type "EngineTypes.EObjectTypeQuery Enum") false (`|MakeArray` (`ActorComponent.GetOwner` (`SceneComponent.GetAttachParent` (`self.K2_GetRootComponent`)))) "ForOneFrame"))
    (if _returnvalue_3
      (`GameplayStatics.ApplyDamage` (`.HitActor` (`GameplayStatics.BreakHitResult` _outhit)) 5.0))))

(event `self.ReceiveAnyDamage`
  (params (Damage :type "Float (single-precision)") (DamageType :type "DamageType Object Reference") (InstigatedBy :type "Controller Object Reference") (DamageCauser :type "Actor Object Reference"))
  (bind _output_get (set `self.CurrentHealth` (- (`self.CurrentHealth`) Damage)))
  (if (<= _output_get 0.0)
    (bind _asbehemoth (cast `/Game/Blueprints/BossFight/Behemoth` (`ActorComponent.GetOwner` (`SceneComponent.GetAttachParent` (`self.K2_GetRootComponent`)))))
    (set `/Game/Blueprints/BossFight/Behemoth.GunsLeft` (- (`/Game/Blueprints/BossFight/Behemoth.GunsLeft` _asbehemoth) 1) _asbehemoth)
    (`self.K2_DestroyActor`)))

(fn `UserConstructionScript`)