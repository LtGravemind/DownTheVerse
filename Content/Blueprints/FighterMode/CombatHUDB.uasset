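; HUD Blueprint for fighter mode that draws a red reticle over the current combat target.
; On each DrawHUD, it projects a valid CurrentTarget's world location to the screen and offsets it to center the square Reticle texture.
; The projected Z value gates drawing, so the reticle only appears when the target is in front of the camera.
; CurrentTarget is only read here, not assigned.
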(event `self.ReceiveBeginPlay`)

(event `self.ReceiveActorBeginOverlap`
  (params (OtherActor :type "Actor Object Reference")))

(event `self.ReceiveTick`
  (params (DeltaSeconds :type "Float (single-precision)")))

(event `self.ReceiveDrawHUD`
  (params (SizeX :type Integer) (SizeY :type Integer))
  (if (`KismetSystemLibrary.IsValid` (`self.CurrentTarget`))
    (if (> (.z (- (`self.Project` (`self.K2_GetActorLocation` (`self.CurrentTarget`))) (25.0 25.0 0.0))) 0.0)
      (`self.DrawTexture` "/Game/Materials/reticle.reticle" (.x (- (`self.Project` (`self.K2_GetActorLocation` (`self.CurrentTarget`))) (25.0 25.0 0.0))) (.y (- (`self.Project` (`self.K2_GetActorLocation` (`self.CurrentTarget`))) (25.0 25.0 0.0))) 50.0 50.0 0.0 0.0 1.0 1.0 (struct :`R` 1.0 :`A` 1.0)))))

(fn `UserConstructionScript`)